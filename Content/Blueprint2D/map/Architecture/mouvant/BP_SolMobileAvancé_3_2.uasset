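; Advanced moving-floor actor (SolMobileAvancé) for a 2D map, built to travel a three-leg loop between Origine, Objectif1 and Objectif2.
; Three chained timelines lerp the actor location along each leg without sweep, ending back at Origine.
; BeginPlay calls Bouger2, which is empty here, and the movement chain hangs off an untriggered Timeline_1, so this graph never moves the floor.
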(event `self.ReceiveBeginPlay`
  (`self.Bouger2`))

(event `Bouger2`)

(fn `UserConstructionScript`)