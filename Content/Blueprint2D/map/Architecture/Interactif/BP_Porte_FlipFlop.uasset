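; Key-locked door actor that moves up to open and down to close.
; TriggerUp and TriggerDown overlaps show press-E or missing-key prompts and, with a key, arm opening or closing respectively.
; GetKey grants the key; MonterPorte and DessendrePorte consume it, hide the key widget and play separate timelines.
; Timelines lerp the actor toward a vertical offset recomputed from Porte's current location each update, then apply the offset again on finish.
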(event `self.TriggerUp.OnComponentBeginOverlap`
  (params (OverlappedComponent :type "PrimitiveComponent Object Reference") (OtherActor :type "Actor Object Reference") (OtherComp :type "PrimitiveComponent Object Reference") (OtherBodyIndex :type Integer) (bFromSweep :type Boolean) (SweepResult :type "HitResult Structure (by ref)"))
  (bind _infoporte (`self.InfoPorte`))
  (if (`self.HaveKey?`)
    (`/Game/Blueprint2D/map/Architecture/Interactif/W_InfoPorte.Press E to oppen W` _infoporte "Visible")
    (set `self.Can oppen` true)
    (else
      (`/Game/Blueprint2D/map/Architecture/Interactif/W_InfoPorte.You don't have the key W` _infoporte "Visible"))))

(event `self.TriggerUp.OnComponentEndOverlap`
  (params (OverlappedComponent :type "PrimitiveComponent Object Reference") (OtherActor :type "Actor Object Reference") (OtherComp :type "PrimitiveComponent Object Reference") (OtherBodyIndex :type Integer))
  (bind _infoporte (`self.InfoPorte`))
  (`/Game/Blueprint2D/map/Architecture/Interactif/W_InfoPorte.You don't have the key W` _infoporte "Collapsed")
  (`/Game/Blueprint2D/map/Architecture/Interactif/W_InfoPorte.Press E to oppen W` _infoporte "Collapsed")
  (set `self.Can oppen` false))

(event `self.TriggerDown.OnComponentBeginOverlap`
  (params (OverlappedComponent :type "PrimitiveComponent Object Reference") (OtherActor :type "Actor Object Reference") (OtherComp :type "PrimitiveComponent Object Reference") (OtherBodyIndex :type Integer) (bFromSweep :type Boolean) (SweepResult :type "HitResult Structure (by ref)"))
  (bind _infoporte (`self.InfoPorte`))
  (if (`self.HaveKey?`)
    (`/Game/Blueprint2D/map/Architecture/Interactif/W_InfoPorte.Press E to oppen W` _infoporte "Visible")
    (set `self.Can close` true)
    (else
      (`/Game/Blueprint2D/map/Architecture/Interactif/W_InfoPorte.You don't have the key W` _infoporte "Visible"))))

(event `self.TriggerDown.OnComponentEndOverlap`
  (params (OverlappedComponent :type "PrimitiveComponent Object Reference") (OtherActor :type "Actor Object Reference") (OtherComp :type "PrimitiveComponent Object Reference") (OtherBodyIndex :type Integer))
  (bind _infoporte (`self.InfoPorte`))
  (`/Game/Blueprint2D/map/Architecture/Interactif/W_InfoPorte.You don't have the key W` _infoporte "Collapsed")
  (`/Game/Blueprint2D/map/Architecture/Interactif/W_InfoPorte.Press E to oppen W` _infoporte "Collapsed")
  (set `self.Can close` false))

(event `Get Key`
  (set `self.HaveKey?` true))

(event `MonterPorte`
  (bind _returnvalue (+ (`SceneComponent.K2_GetComponentLocation` (`self.Porte`)) (0.0 0.0 230.0)))
  ;[1 1 1] Monter
  (if (`self.Can oppen`)
    (set `self.HaveKey?` false)
    (`/Game/Blueprint2D/map/Architecture/Interactif/W_InfoKey.Info Key W` (`self.Info key`) "Collapsed")
    (bind (_direction _float) (`Timeline|Timeline`)
      (:`Update`
        (`self.K2_SetActorLocation` (`KismetMathLibrary.VLerp` (`SceneComponent.K2_GetComponentLocation` (`self.Porte`)) _returnvalue _float)))
      (:`Finished`
        (`self.K2_SetActorLocation` _returnvalue)))))

(event `DessendrePorte`
  (bind _returnvalue (+ (`SceneComponent.K2_GetComponentLocation` (`self.Porte`)) (0.0 0.0 -230.0)))
  ;[1 1 1] Dessendre
  (if (`self.Can close`)
    (set `self.HaveKey?` false)
    (`/Game/Blueprint2D/map/Architecture/Interactif/W_InfoKey.Info Key W` (`self.Info key`) "Collapsed")
    (bind (_direction _float) (`Timeline|Timeline_0`)
      (:`Update`
        (`self.K2_SetActorLocation` (`KismetMathLibrary.VLerp` (`SceneComponent.K2_GetComponentLocation` (`self.Porte`)) _returnvalue _float)))
      (:`Finished`
        (`self.K2_SetActorLocation` _returnvalue)))))

(fn `UserConstructionScript`)